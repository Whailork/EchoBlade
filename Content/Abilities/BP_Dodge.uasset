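; Dodge ability that rolls a Fighter, playing a montage and locking player input until the ability stops.
; On start it builds a yaw-relative roll vector from player movement input, or a random backward-to-sideways one for other fighters.
; A looping timer applies that vector as movement force and rotates the mesh toward it through a DoOnce.
; Stopping restores input and mesh rotation and resets the DoOnce; no timer clear is shown.
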(event Custom|AddForce
  (bind _rollvector (Variables|Default|GetRollVector))
  (bind _returnvalue (Math|Conversions|RotationFromXVector _rollvector))
  (Physics|AddForce (Variables|/Script/Engine.Character|GetCharacterMovement (Variables|Default|GetFighter)) (Variables|Default|GetRollVector))
  (if (Utilities|Operators|NotEqual(!=) (Transformation|GetActorRotation (Variables|Default|GetFighter)) _returnvalue 1e+01)
    (Utilities|FlowControl|DoOnce false
      (:Completed
        (Transformation|AddRelativeRotation (Variables|/Script/Engine.Character|GetMesh (Variables|Default|GetFighter)) _returnvalue false false)))))

(event EventOnAbilityStarted
  (params (instigator :type Actor%20Object%20Reference))
  (bind _rollforce (Variables|Default|GetRollForce))
  (bind _rollforce_2 (Variables|Default|GetRollForce))
  (bind _asfighter (Utilities|Casting|CastToFighter instigator))
  (Variables|Default|SetFighter _asfighter)
  (Animation|PlayAnimMontage _asfighter "/Game/Animations/Roll/DodgeMontage.DodgeMontage" 1.0 "None")
  (bind _asplayer_controller (Utilities|Casting|CastToPlayerController (Pawn|GetController _asfighter))
    (:then
      (Input|DisableInput _asfighter _asplayer_controller))
    (:CastFailed
      _))
  (Variables|Default|SetBaseRotation (Variables|/Script/Engine.SceneComponent|GetRelativeRotation (Variables|/Script/Engine.Character|GetMesh (Variables|Default|GetFighter))))
  (bind _asplayer_fighter (Utilities|Casting|CastToPlayerFighter (Variables|Default|GetFighter))
    (:then
      (Variables|Default|SetRollVector (+ (* (Math|Vector|GetForwardVector (Math|Rotator|MakeRotator 0.0 0.0 (.Yaw (Math|Rotator|BreakRotator (Pawn|GetControlRotation (Variables|Default|GetFighter) :!class /Script/Engine.Pawn))))) _rollforce (.y (Math|Vector2D|Normalize2D (Variables|/Script/EchoBlade.PlayerFighter|GetMovementVector _asplayer_fighter)))) (* (Math|Vector|GetRightVector (Math|Rotator|MakeRotator 0.0 0.0 (.Yaw (Math|Rotator|BreakRotator (Pawn|GetControlRotation (Variables|Default|GetFighter) :!class /Script/Engine.Pawn))))) (.x (Math|Vector2D|Normalize2D (Variables|/Script/EchoBlade.PlayerFighter|GetMovementVector _asplayer_fighter))) _rollforce))))
    (:CastFailed
      (Variables|Default|SetRollVector (+ (* (Math|Vector|GetForwardVector (Math|Rotator|MakeRotator 0.0 0.0 (.Yaw (Math|Rotator|BreakRotator (Pawn|GetControlRotation (Variables|Default|GetFighter) :!class /Script/Engine.Pawn))))) _rollforce_2 (Math|Random|RandomFloatinRange -1.0 0.0)) (* (Math|Vector|GetRightVector (Math|Rotator|MakeRotator 0.0 0.0 (.Yaw (Math|Rotator|BreakRotator (Pawn|GetControlRotation (Variables|Default|GetFighter) :!class /Script/Engine.Pawn))))) (Math|Random|RandomFloatinRange -1.0 1.0) _rollforce_2)))))
  (bind _returnvalue (Utilities|Time|SetTimerbyEvent (delegate Custom|AddForce) 0.05 true))
  (Variables|Default|SetTimerHandle _returnvalue))

(event EventOnAbilityStopped
  (params (instigator :type Actor%20Object%20Reference))
  (bind _fighter (Variables|Default|GetFighter))
  (bind _asplayer_controller (Utilities|Casting|CastToPlayerController (Pawn|GetController _fighter))
    (:then
      (Input|EnableInput _fighter _asplayer_controller))
    (:CastFailed
      _))
  (Transformation|SetRelativeRotation (Variables|/Script/Engine.Character|GetMesh (Variables|Default|GetFighter)) (Variables|Default|GetBaseRotation) false false)
  (Utilities|FlowControl|Sequence
    (:then_0
      (Utilities|FlowControl|DoOnce false) ; enters at Reset
    )))

(fn BeginRollMovement
  (params (Force :type Float%20%28double-precision%29))
  (bind _fighter (Variables|Default|GetFighter))
  (bind _returnvalue (Transformation|GetVelocity _fighter))
  (bind _returnvalue_2 (Math|Vector|Normalize _returnvalue))
  (if (> (Math|Vector|VectorLength _returnvalue) 1e+01)
    (Physics|AddForce (Variables|/Script/Engine.Character|GetCharacterMovement _fighter) (* _returnvalue_2 Force))
    (Utilities|FlowControl|DoOnce false
      (:Completed
        (Transformation|AddRelativeRotation (Variables|/Script/Engine.Character|GetMesh _fighter) (Math|Conversions|RotationFromXVector _returnvalue_2) false false)
        (return)))))

(fn StopRolling)