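; BP_WindGustAbility is a gameplay ability that launches nearby enemy fighters away from the player.
; On activation it temporarily widens the player's capsule to BlowRadius, using its overlaps as the area query for BP_EnemyFighter actors.
; Each enemy is launched along the normalized direction from the player with reduced vertical force, then the capsule radius is restored and the ability ends.
; GetPlayer resolves the avatar as BP_PlayerFighter only with authority.
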(event Ability|EventActivateAbility
  (bind _asbp_player_fighter (CallFunction|GetPlayer))
  (Variables|Default|SetPlayerLocation (Transformation|GetActorLocation _asbp_player_fighter))
  (Variables|Default|SetPlayerCapsule (Actor|GetComponentbyClass _asbp_player_fighter "/Script/Engine.CapsuleComponent"))
  (Variables|Default|SetInitialCapsuleRadius (Variables|/Script/Engine.CapsuleComponent|GetCapsuleRadius (Variables|Default|GetPlayerCapsule)))
  (Components|Capsule|SetCapsuleRadius (Variables|Default|GetPlayerCapsule) (Variables|Default|GetBlowRadius) true)
  (for _array_element (Collision|GetOverlappingActors (Variables|Default|GetPlayerCapsule) "/Game/Blueprints/BP_EnemyFighter.BP_EnemyFighter_C" :!class /Script/Engine.PrimitiveComponent)
    (bind _asbp_enemy_fighter (Utilities|Casting|CastToBP_EnemyFighter _array_element))
    (Variables|Default|SetCurrentEnemyLocation (Transformation|GetActorLocation _asbp_enemy_fighter))
    (Character|LaunchCharacter _asbp_enemy_fighter (* (Math|Vector|Normalize (- (Variables|Default|GetCurrentEnemyLocation) (Variables|Default|GetPlayerLocation))) "100.000000,100.000000,10.000000") true true))
  (Components|Capsule|SetCapsuleRadius (Variables|Default|GetPlayerCapsule) (Variables|Default|GetInitialCapsuleRadius) true)
  (Class|EchoBladeGameplayAbility|EchoEndAbility))

(event Ability|EventOnEndAbility
  (params (bWasCancelled :type Boolean)))

(fn GetPlayer
  (Ability|HasAuthority
    (:True
      (bind _returnvalue (Class|EchoBladeGameplayAbility|GetActorInfoTemp))
      (bind _asbp_player_fighter (Utilities|Casting|CastToBP_PlayerFighter (.avataractor _returnvalue)))
      (return _asbp_player_fighter))))