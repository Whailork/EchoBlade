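; BP_InstantHeal is a gameplay ability that heals the avatar's Health in a near-instant burst.
; On activation with authority, it reads values from the avatar's AttributeSystemComponent.
; It adds a Regeneration effect with a tiny period, whose power is current value plus half max Health, clamped to the attribute bounds.
; The ability then ends through EchoEndAbility.
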(event Ability|EventActivateAbility
  (Ability|HasAuthority
    (:True
      (bind _returnvalue (Class|EchoBladeGameplayAbility|GetActorInfoTemp))
      (Utilities|IsValid (Actor|GetComponentbyClass (.avataractor _returnvalue) "/Script/FASAttribute.AttributeSystemComponent")
        (:Is%20Valid
          (bind _outvalue (Class|AttributeSystemComponent|GetAttributeMaxValue (Actor|GetComponentbyClass (.avataractor _returnvalue) "/Script/FASAttribute.AttributeSystemComponent") "(TagName=\"Attribute.Health\")"))
          (bind _outvalue_2 (Class|AttributeSystemComponent|GetAttributeValue (Actor|GetComponentbyClass (.avataractor _returnvalue) "/Script/FASAttribute.AttributeSystemComponent")))
          (bind _outvalue_3 (Class|AttributeSystemComponent|GetAttributeMinValue (Actor|GetComponentbyClass (.avataractor _returnvalue) "/Script/FASAttribute.AttributeSystemComponent")))
          (bind _returnvalue_2 (Game|ConstructObjectfromClass (.avataractor _returnvalue) "/Script/EchoBlade.Regeneration"))
          (Class|CustomGameplayEffect|InitializeValues _returnvalue_2 0.0 0.0001 "(TagName=\"Attribute.Health\")" (Math|Float|Clamp(Float) (+ _outvalue_2 (/ _outvalue 2.0)) _outvalue_3 _outvalue) false false)
          (Class|AttributeSystemComponent|AddEffect (Actor|GetComponentbyClass (.avataractor _returnvalue) "/Script/FASAttribute.AttributeSystemComponent") _returnvalue_2))
        (:Is%20Not%20Valid
          _))
      (Class|EchoBladeGameplayAbility|EchoEndAbility))))