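; Fireball ability that fires a fire-material projectile with a linked Hit effect from the instigating Fighter, then stops immediately.
; Activation starts the cooldown, calls ChangeOpacity and runs a looping one-second timer that counts down into the player's Skill 1 HUD text.
; At zero the timer handle is only invalidated, not cleared.
; CanStartAbility ignores the parent's result, gating solely on ImageTop's render opacity being zero.
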(event Custom|StartCooldown
  (Variables|Default|SetCooldownRemaining (Variables|Default|GetAbilityCooldown))
  (Class|Ability|ChangeOpacity)
  (bind _returnvalue (Utilities|Time|SetTimerbyFunctionName 0 (Variables|Default|GetUpdateCooldownName) 1.0 true))
  (Variables|Default|SetCooldownTimer _returnvalue))

(event Custom|UpdateCooldown
  (if (not (== (Variables|Default|GetCooldownRemaining) 0.0))
    (bind _asbp_player_fighter (Utilities|Casting|CastToBP_PlayerFighter (Variables|Default|GetInstigator)))
    (Variables|/Game/UI/WBP_Layout_06.WBP_Layout_06_C|SetSkill_1_Cooldown_Text (Variables|/Game/Blueprints/BP_PlayerFighter.BP_PlayerFighter_C|GetWidgetLayout06 _asbp_player_fighter) (Utilities|Text|ToText(Float) (Variables|Default|GetCooldownRemaining) "HalfToEven"))
    (Math|Float|DecrementFloat (Variables|Default|GetCooldownRemaining))
    (else
      (Utilities|Time|InvalidateTimerHandle (Variables|Default|GetCooldownTimer)))))

(event EventOnAbilityStarted
  (params (instigator :type Actor%20Object%20Reference))
  (Variables|Default|SetInstigator instigator)
  (CallFunction|StartCooldown)
  (bind _asfighter (Utilities|Casting|CastToFighter instigator))
  (Class|Fighter|SpawnProjectile _asfighter _asfighter "/Game/FXVarietyPack/Materials/MI_ky_storm01_fire.MI_ky_storm01_fire" "/Script/EchoBlade.Hit")
  (Class|Ability|Stop _asfighter false))

(fn CanStartAbility
  (params (instigator :type Actor%20Object%20Reference))
  (|CallParentFunction instigator)
  (return (== (Class|Widget|GetRenderOpacity (Variables|Default|GetImageTop)) 0.0)))